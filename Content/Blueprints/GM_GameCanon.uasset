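; Game mode for a cannon-launch obstacle game, running the flow from start screen to victory or death.
; The start input caches key actors and plays a launch cinematic, optionally sped up, whose end activates the player, collision box and obstacle spawner.
; FinishGame shows a victory widget on hitting BP_KayouFinal, otherwise fades out, with timers to reset the level.
; An optional render-target widget is added at startup.
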(event Input|EnhancedActionEvents|EnhancedInputActionIA_StartGame
  (params (ActionValue :type Boolean) (ElapsedSeconds :type Float%20%28double-precision%29) (TriggeredSeconds :type Float%20%28double-precision%29) (InputAction :type Input%20Action%20Object%20Reference :default "/Game/ThirdPerson/Input/Actions/IA_StartGame.IA_StartGame"))
  (Utilities|FlowControl|DoOnce false
    (:Completed
      (CallFunction|StartGame)
      (Widget|RemovefromParent (Variables|Default|GetWG_StartScreen)))))

(event EventBeginPlay
  (Input|EnableInput (Game|GetPlayerController 0))
  (bind _returnvalue (UserInterface|CreateWidget "/Game/UI/WB_StartScreen.WB_StartScreen_C"))
  (Variables|Default|SetWG_StartScreen _returnvalue)
  (if (Variables|Default|GetAddWidget360_)
    (CallFunction|ADDWidget360))
  (UserInterface|Viewport|AddtoViewport (Variables|Default|GetWG_StartScreen) 0))

(fn ConstructionScript)

(fn LaunchStartCinematic
  (bind _returnvalue (Sequencer|Player|CreateLevelSequencePlayer (Variables|Cinematic|GetLevelSequence)))
  (Variables|Cinematic|SetLevelSequencePlayer _returnvalue)
  (EventDispatchers|BindEventtoOnStop (Variables|Cinematic|GetLevelSequencePlayer) (EventDispatchers|CreateEvent :!event EndStartCinematic))
  (if (Variables|Cinematic|GetSkipCinematic?)
    (Components|Timeline|SetPlayRate (Variables|Cinematic|GetLevelSequencePlayer) 1e+01))
  (Sequencer|Player|Play (Variables|Cinematic|GetLevelSequencePlayer) :!class /Script/MovieScene.MovieSceneSequencePlayer)
  (Default|StartRotation (Variables|Default|GetPlayer))
  (Default|StartThrottle (Variables|Default|GetPlayer))
  (Default|PlaySoundLaunch (Variables|Default|GetBP_Canon))
  (Default|PlayMusic (Variables|Default|GetBP_KayouFinal)))

(fn StartGame
  (bind _returnvalue (Actor|GetActorOfClass "/Game/ThirdPerson/Blueprints/BP_ThirdPersonCharacter.BP_ThirdPersonCharacter_C"))
  (Variables|Default|SetPlayer _returnvalue)
  (bind _returnvalue_2 (Actor|GetActorOfClass "/Game/Blueprints/CollisionBoxPlayer.CollisionBoxPlayer_C"))
  (Variables|Default|SetCollisionBoxPlayer _returnvalue_2)
  (bind _returnvalue_3 (Actor|GetActorOfClass "/Game/Blueprints/BP_ObstacleSpawner.BP_ObstacleSpawner_C"))
  (Variables|Default|SetObstacleSpawner _returnvalue_3)
  (bind _returnvalue_4 (Actor|GetActorOfClass "/Game/Blueprints/BP_Canon.BP_Canon_C"))
  (Variables|Default|SetBP_Canon _returnvalue_4)
  (bind _returnvalue_5 (Actor|GetActorOfClass "/Game/Blueprints/Obstacle/BP_KayouFinal.BP_KayouFinal_C"))
  (Variables|Default|SetBP_KayouFinal _returnvalue_5)
  (CallFunction|LaunchStartCinematic))

(fn EndStartCinematic
  (Default|StartGame (Variables|Default|GetPlayer))
  (Default|StartGame (Variables|Default|GetCollisionBoxPlayer))
  (Default|SetActive (Variables|Default|GetObstacleSpawner) true))

(fn FinishGame
  (params (LocalCollideActor :type Actor%20Object%20Reference))
  (Utilities|Casting|CastToBP_KayouFinal LocalCollideActor
    (:then
      (CallFunction|Victory))
    (:CastFailed
      (CameraFades|StartCameraFade :self (Variables|/Script/Engine.PlayerController|GetPlayerCameraManager (Game|GetPlayerController 0)) :ToAlpha 1.0 :Duration (Variables|Default|GetDurationFadeDeath) :bShouldFadeAudio true :bHoldWhenFinished true)
      (Utilities|Time|SetTimerbyEvent (EventDispatchers|CreateEvent :!event RestartLevel) (+ (Variables|Default|GetDurationFadeDeath) (Variables|Default|GetDelayRestartGame)) false true))))

(fn RestartLevel
  (bind _returnvalue (Game|GetCurrentLevelName true))
  (Game|OpenLevel(byName) (Utilities|String|StringToName _returnvalue)))

(fn ADDWidget360
  (bind _returnvalue (UserInterface|CreateWidget "/Game/UI/WG_RenderTarget.WG_RenderTarget_C"))
  (UserInterface|Viewport|AddtoViewport _returnvalue 0))

(fn Victory
  (bind _returnvalue (UserInterface|CreateWidget "/Game/UI/WG_Victory.WG_Victory_C"))
  (UserInterface|Viewport|AddtoViewport _returnvalue 0)
  (Utilities|Time|SetTimerbyEvent (EventDispatchers|CreateEvent :!event RestartLevel) (Variables|Default|GetDelayVictoryReset) false true))