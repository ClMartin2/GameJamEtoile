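; BP_Kayou2 is a destructible obstacle that shatters through Chaos when something begins overlapping its OverlapChaos trigger.
; The overlap enables physics on the GCKayou2RTP component and spawns an FS_MasterFieldCustom field actor at the obstacle's transform.
; It then calls TouchObstacle on the player's BP_ThirdPersonCharacter and stops SoundProxiPlayer.
; The overlapping actor is not checked; player character 0 is always notified.
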(event OnComponentBeginOverlap(OverlapChaos)
  (params (OverlappedComponent :type Primitive%20Component%20Object%20Reference) (OtherActor :type Actor%20Object%20Reference) (OtherComp :type Primitive%20Component%20Object%20Reference) (OtherBodyIndex :type Integer) (bFromSweep :type Boolean) (SweepResult :type Hit%20Result%20Structure%20%28by%20ref%29))
  (Physics|SetSimulatePhysics (Variables|Default|GetGC_Kayou2RTP) true)
  (Game|SpawnActorfromClass "/Game/Chaos/FS_MasterFieldCustom.FS_MasterFieldCustom_C" (Transformation|GetActorTransform) "Undefined" "MultiplyWithRoot" 0 0)
  (bind _asbp_third_person_character (Utilities|Casting|CastToBP_ThirdPersonCharacter (Game|GetPlayerCharacter 0)))
  (Default|TouchObstacle _asbp_third_person_character self)
  (Audio|Components|Audio|Stop (Variables|Default|GetSoundProxiPlayer)))

(fn ConstructionScript
  (|CallParentFunction))