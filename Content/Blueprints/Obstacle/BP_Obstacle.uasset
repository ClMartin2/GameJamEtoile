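; BP_Obstacle is a moving obstacle actor that travels along its forward vector while its Kayou1RTP component tumbles.
; BeginPlay picks a random rotation axis.
; Tick moves the actor by MoveSpeed without sweeping, then applies a jittered local rotation around that axis, with the whole accumulated angle scaled by delta time each frame.
; Initialize, Destroy and the construction script are empty.
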(event EventBeginPlay
  (Variables|Default|SetRotationAxis (Math|Random|RandomUnitVector)))

(event EventTick
  (params (DeltaSeconds :type Float%20%28single-precision%29))
  (bind _rotationspeed (Variables|Default|GetRotationSpeed))
  (Transformation|SetActorLocation (+ (* DeltaSeconds (* (Transformation|GetActorForwardVector) (Variables|Default|GetMoveSpeed))) (Transformation|GetActorLocation)) false false)
  (bind _output_get (Variables|Default|SetCurrentAngle (* (+ (Variables|Default|GetCurrentAngle) (Math|Random|RandomFloatinRange (- _rotationspeed 8.0) (+ _rotationspeed 8.0))) DeltaSeconds)))
  (Transformation|AddLocalRotation (Variables|Default|GetKayou1RTP) (Math|Vector|RotatorfromAxisandAngle (Variables|Default|GetRotationAxis) _output_get) false false))

(fn ConstructionScript)

(fn Initialize)

(fn Destroy)