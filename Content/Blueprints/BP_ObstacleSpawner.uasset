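; Obstacle spawner actor that emits a sequence of difficulty-tiered phase actors facing the player.
; Initialize places it at a set distance along the player's rotated forward vector plus a fixed offset, after a startup delay and whenever SetActive enables it.
; While active, a Delay on Tick paces spawning as PhaseCounter steps through AllPhases, picking a random class from each tier's list.
; SpawnObstacle, unused here, spawns a given class at a random radial offset.
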(event EventTick
  (params (DeltaSeconds :type Float%20%28single-precision%29))
  (if (Variables|Default|GetisInitiated)
    (if (Variables|Default|GetisActive)
      (Utilities|FlowControl|Delay (Variables|Default|GetSpawnRate))
      (switch Utilities|FlowControl|Switch|SwitchonGamePhases (Utilities|Array|Get(acopy) (Variables|Default|GetAllPhases) (Variables|Default|GetPhaseCounter))
        (:NewEnumerator0
          (CallFunction|SpawnPhase (Variables|Default|GetEasyPhase)))
        (:NewEnumerator1
          (CallFunction|SpawnPhase (Variables|Default|GetMediumPhase)))
        (:NewEnumerator2
          (CallFunction|SpawnPhase (Variables|Default|GetHardPhase)))
        (:NewEnumerator3
          (CallFunction|SpawnPhase (Variables|Default|GetWowPhase))))
      (Math|Integer|IncrementInt (Variables|Default|GetPhaseCounter)))
    (else
      (Utilities|FlowControl|Delay 1.5)
      (CallFunction|Initialize)
      (Variables|Default|SetisInitiated true))))

(fn ConstructionScript)

(fn SpawnObstacle
  (params (ClassToSpawn :type BP%20Obstacle%20Class%20Reference))
  (bind _returnvalue (Transformation|GetActorTransform))
  (Game|SpawnActorfromClass ClassToSpawn (Math|Transform|MakeTransform (+ (* (Math|Random|RandomUnitVector) (Variables|Default|GetMaxSpawnRadius)) (.location _returnvalue)) (.rotation _returnvalue)) "Undefined" "MultiplyWithRoot" 0 0))

(fn Initialize
  (Transformation|SetActorLocation (+ (* (Math|Vector|Normalize (Math|Vector|RotateVectorAroundAxis (Transformation|GetActorForwardVector (Variables|Default|GetPlayer)) (Variables|Default|GetLevelMovementAngle) "1.000000,0.000000,0.000000")) (Variables|Default|GetDistanceToPlayer)) "0.000000,-4000.000000,0.000000") false false)
  (Transformation|SetActorRotation (Math|Rotator|FindLookatRotation (Transformation|GetActorLocation) (Transformation|GetActorLocation (Variables|Default|GetPlayer)))))

(fn SetActive
  (params (value :type Boolean))
  (bind _output_get (Variables|Default|SetisActive value))
  (if _output_get
    (CallFunction|Initialize)))

(fn SpawnPhase
  (params (NewParam :type Array%20of%20BP%20Phase%20Class%20References))
  (bind _returnvalue (Transformation|GetActorTransform))
  (Game|SpawnActorfromClass (.OutItem (Utilities|Array|Random NewParam)) (Math|Transform|MakeTransform (.location _returnvalue) (.rotation _returnvalue)) "Undefined" "MultiplyWithRoot" 0 0))